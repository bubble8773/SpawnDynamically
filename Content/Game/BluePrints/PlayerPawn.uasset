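; Player pawn for grid movement, stepping between linked tiles via WASD or matching Move events.
; Input is gated by CanMoveOverride and an empty TargetTile, then looks up the neighbour and starts timeline-driven position and rotation lerps.
; Tiles control entry through CanPlayerEnter, can chain automatic moves through GetNextTile, and receive OnEntered on arrival.
; OpenNextLevel opens a fixed level, L3; its LevelList lookup is unconnected.
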(event Custom|MoveToTile
  (params (TileToMoveTo :type Tile%20Object%20Reference))
  ;[1 1 1] Movement and Rotation
  (Utilities|IsValid TileToMoveTo
    (:Is%20Valid
      (if (Default|CanPlayerEnter TileToMoveTo self (Variables|Default|GetCurrentTile))
        (Variables|Default|SetTargetTile TileToMoveTo)
        (bind _moveprogress (Timeline|MovementTimeline PlayFromStart)
          (:Update
            (Transformation|SetActorLocation (Math|Vector|Lerp(Vector) (Transformation|GetActorLocation (Variables|Default|GetCurrentTile)) (Transformation|GetActorLocation TileToMoveTo) _moveprogress) false false))
          (:Finished
            (Variables|Default|SetTemp (Variables|Default|GetCurrentTile))
            (Variables|Default|SetCurrentTile (Variables|Default|GetTargetTile))
            (bind _output_get (Variables|Default|SetTargetTile (Default|GetNextTile (Variables|Default|GetCurrentTile) self (Variables|Default|GetTemp))))
            (Utilities|IsValid _output_get
              (:Is%20Valid
                (if (Default|CanPlayerEnter _output_get self (Variables|Default|GetCurrentTile))
                  (CallFunction|MovetoTile (Variables|Default|GetTargetTile))
                  (else
                    (Variables|Default|SetTargetTile 0))))
              (:Is%20Not%20Valid
                _))
            (Default|OnEntered (Variables|Default|GetCurrentTile) self (Variables|Default|GetTemp))))))))

(event Custom|MoveUp
  (bind _currenttile (Variables|Default|GetCurrentTile))
  (bind _neighbours (Variables|/Game/Game/BluePrints/TileManagement/Tile.Tile_C|GetNeighbours _currenttile))
  (bind _value (Utilities|Map|Find _neighbours "/Game/Game/Data/Up.Up"))
  ;[1 1 1] MoveUp
  (if (Variables|Default|GetCanMoveOverride)
    (Utilities|IsValid (Variables|Default|GetTargetTile)
      (:Is%20Not%20Valid
        (Utilities|IsValid _value
          (:Is%20Valid
            (CallFunction|MovetoTile _value)
            (CallFunction|RotatetoDirection "/Game/Game/Data/Up.Up")))))))

(event Custom|MoveRight
  (bind _currenttile (Variables|Default|GetCurrentTile))
  (bind _neighbours (Variables|/Game/Game/BluePrints/TileManagement/Tile.Tile_C|GetNeighbours _currenttile))
  (bind _value (Utilities|Map|Find _neighbours "/Game/Game/Data/Right.Right"))
  ;[1 1 1] MoveRight
  (if (Variables|Default|GetCanMoveOverride)
    (Utilities|IsValid (Variables|Default|GetTargetTile)
      (:Is%20Not%20Valid
        (Utilities|IsValid _value
          (:Is%20Valid
            (CallFunction|MovetoTile _value)
            (CallFunction|RotatetoDirection "/Game/Game/Data/Right.Right")))))))

(event Custom|MoveDown
  (bind _currenttile (Variables|Default|GetCurrentTile))
  (bind _neighbours (Variables|/Game/Game/BluePrints/TileManagement/Tile.Tile_C|GetNeighbours _currenttile))
  (bind _value (Utilities|Map|Find _neighbours "/Game/Game/Data/Down.Down"))
  ;[1 1 1] MoveDown
  (if (Variables|Default|GetCanMoveOverride)
    (Utilities|IsValid (Variables|Default|GetTargetTile)
      (:Is%20Not%20Valid
        (Utilities|IsValid _value
          (:Is%20Valid
            (CallFunction|MovetoTile _value)
            (CallFunction|RotatetoDirection "/Game/Game/Data/Down.Down")))))))

(event Custom|MoveLeft
  (bind _currenttile (Variables|Default|GetCurrentTile))
  (bind _neighbours (Variables|/Game/Game/BluePrints/TileManagement/Tile.Tile_C|GetNeighbours _currenttile))
  (bind _value (Utilities|Map|Find _neighbours "/Game/Game/Data/Left.Left"))
  ;[1 1 1] MoveLeft
  (if (Variables|Default|GetCanMoveOverride)
    (Utilities|IsValid (Variables|Default|GetTargetTile)
      (:Is%20Not%20Valid
        (Utilities|IsValid _value
          (:Is%20Valid
            (CallFunction|MovetoTile _value)
            (CallFunction|RotatetoDirection "/Game/Game/Data/Left.Left")))))))

(event Custom|RotateToDirection
  (params (Direction :type Direction%20Object%20Reference))
  ;[1 1 1] Movement and Rotation
  (Utilities|IsValid Direction
    (:Is%20Valid
      (Variables|Default|SetTargetDirection Direction)
      (bind _rotateprogress (Timeline|RotateToTimeline PlayFromStart)
        (:Update
          (Transformation|SetActorRotation (Math|Rotator|Lerp(Rotator) (Variables|/Game/Game/Data/Direction.Direction_C|GetRotation (Variables|Default|GetCurrentDirection)) (Variables|/Game/Game/Data/Direction.Direction_C|GetRotation (Variables|Default|GetTargetDirection)) _rotateprogress true)))
        (:Finished
          (Variables|Default|SetCurrentDirection (Variables|Default|GetTargetDirection))
          (Variables|Default|SetTargetDirection 0))))))

(event EventBeginPlay)

(event Collision|EventActorBeginOverlap
  (params (OtherActor :type Actor%20Object%20Reference)))

(event EventTick
  (params (DeltaSeconds :type Float%20%28single-precision%29)))

(event Input|ActionEvents|InputActionIMoveUp
  (params (Key :type Key%20Structure :default "None")))

(event Input|ActionEvents|InputActionIMoveRight
  (params (Key :type Key%20Structure :default "None")))

(event Input|ActionEvents|InputActionIMoveLeft
  (params (Key :type Key%20Structure :default "None")))

(event Input|KeyboardEvents|W
  (params (Key :type Key%20Structure :default "None"))
  (bind _currenttile (Variables|Default|GetCurrentTile))
  (bind _neighbours (Variables|/Game/Game/BluePrints/TileManagement/Tile.Tile_C|GetNeighbours _currenttile))
  (bind _value (Utilities|Map|Find _neighbours "/Game/Game/Data/Up.Up"))
  ;[1 1 1] MoveUp
  (:Pressed
    (if (Variables|Default|GetCanMoveOverride)
      (Utilities|IsValid (Variables|Default|GetTargetTile)
        (:Is%20Not%20Valid
          (Utilities|IsValid _value
            (:Is%20Valid
              (CallFunction|MovetoTile _value)
              (CallFunction|RotatetoDirection "/Game/Game/Data/Up.Up"))))))))

(event Input|KeyboardEvents|A
  (params (Key :type Key%20Structure :default "None"))
  (bind _currenttile (Variables|Default|GetCurrentTile))
  (bind _neighbours (Variables|/Game/Game/BluePrints/TileManagement/Tile.Tile_C|GetNeighbours _currenttile))
  (bind _value (Utilities|Map|Find _neighbours "/Game/Game/Data/Left.Left"))
  ;[1 1 1] MoveLeft
  (:Pressed
    (if (Variables|Default|GetCanMoveOverride)
      (Utilities|IsValid (Variables|Default|GetTargetTile)
        (:Is%20Not%20Valid
          (Utilities|IsValid _value
            (:Is%20Valid
              (CallFunction|MovetoTile _value)
              (CallFunction|RotatetoDirection "/Game/Game/Data/Left.Left"))))))))

(event Input|KeyboardEvents|S
  (params (Key :type Key%20Structure :default "None"))
  (bind _currenttile (Variables|Default|GetCurrentTile))
  (bind _neighbours (Variables|/Game/Game/BluePrints/TileManagement/Tile.Tile_C|GetNeighbours _currenttile))
  (bind _value (Utilities|Map|Find _neighbours "/Game/Game/Data/Down.Down"))
  ;[1 1 1] MoveDown
  (:Pressed
    (if (Variables|Default|GetCanMoveOverride)
      (Utilities|IsValid (Variables|Default|GetTargetTile)
        (:Is%20Not%20Valid
          (Utilities|IsValid _value
            (:Is%20Valid
              (CallFunction|MovetoTile _value)
              (CallFunction|RotatetoDirection "/Game/Game/Data/Down.Down"))))))))

(event Input|KeyboardEvents|D
  (params (Key :type Key%20Structure :default "None"))
  (bind _currenttile (Variables|Default|GetCurrentTile))
  (bind _neighbours (Variables|/Game/Game/BluePrints/TileManagement/Tile.Tile_C|GetNeighbours _currenttile))
  (bind _value (Utilities|Map|Find _neighbours "/Game/Game/Data/Right.Right"))
  ;[1 1 1] MoveRight
  (:Pressed
    (if (Variables|Default|GetCanMoveOverride)
      (Utilities|IsValid (Variables|Default|GetTargetTile)
        (:Is%20Not%20Valid
          (Utilities|IsValid _value
            (:Is%20Valid
              (CallFunction|MovetoTile _value)
              (CallFunction|RotatetoDirection "/Game/Game/Data/Right.Right"))))))))

(fn ConstructionScript)

(fn OpenNextLevel
  (Game|OpenLevel(byObjectReference) "/Game/Game/Maps/L3.L3"))