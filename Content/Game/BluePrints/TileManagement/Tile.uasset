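; Base tile actor for a coordinate grid owned by a TileMap, with stub hooks for player entry, entered events and next-tile lookup; entry is refused by default.
; FindNeighbours queries the map in four directions and caches valid tiles by direction.
; ChangeTileType swaps the tile by spawning the new class with the same state, relinking neighbours through opposite directions, updating the map and destroying itself.
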(event Custom|OnEntered
  (params (Player :type Player%20Pawn%20Object%20Reference) (From :type Tile%20Object%20Reference)))

(event EventBeginPlay)

(event Collision|EventActorBeginOverlap
  (params (OtherActor :type Actor%20Object%20Reference)))

(event EventTick
  (params (DeltaSeconds :type Float%20%28single-precision%29)))

(fn ConstructionScript)

(fn FindNeighbours
  (bind _coord (Variables|Default|GetCoord))
  (for _array_element (Utilities|Array|MakeArray "/Game/Game/Data/Up.Up" "/Game/Game/Data/Down.Down" "/Game/Game/Data/Left.Left" "/Game/Game/Data/Right.Right")
    (if (Default|IsCoordinRange (Variables|Default|GetTileMapRef) (Utilities|Struct|MakeCoord (+ (.x (Variables|/Game/Game/Data/Direction.Direction_C|GetDelta _array_element)) (.x _coord)) (+ (.y (Variables|/Game/Game/Data/Direction.Direction_C|GetDelta _array_element)) (.y _coord))))
      (Utilities|IsValid (Default|GetTileatCoord (Variables|Default|GetTileMapRef) (Utilities|Struct|MakeCoord (+ (.x (Variables|/Game/Game/Data/Direction.Direction_C|GetDelta _array_element)) (.x _coord)) (+ (.y (Variables|/Game/Game/Data/Direction.Direction_C|GetDelta _array_element)) (.y _coord))))
        (:Is%20Valid
          (Utilities|Map|Add (Variables|Default|GetNeighbours) _array_element (Default|GetTileatCoord (Variables|Default|GetTileMapRef) (Utilities|Struct|MakeCoord (+ (.x (Variables|/Game/Game/Data/Direction.Direction_C|GetDelta _array_element)) (.x _coord)) (+ (.y (Variables|/Game/Game/Data/Direction.Direction_C|GetDelta _array_element)) (.y _coord))))))))))

(fn ChangeTileType
  (bind _newtiletype (Variables|Default|GetNewTileType))
  (bind _newtiletype_2 (Variables|Default|GetNewTileType))
  (if (and (Utilities|IsValidClass _newtiletype) (!= _newtiletype (Utilities|GetClass self)))
    (bind _returnvalue (Game|SpawnActorfromClass _newtiletype_2 (Transformation|GetActorTransform) "AlwaysSpawn" 0 _newtiletype_2 (Variables|Default|GetCoord) (Variables|Default|GetNeighbours) (Variables|Default|GetTileMapRef) 0))
    (bind _keys (Utilities|Map|Keys (Variables|Default|GetNeighbours)))
    (for _array_element _keys
      (Utilities|IsValid (.Value (Utilities|Map|Find (Variables|Default|GetNeighbours) _array_element))
        (:Is%20Valid
          (CallFunction|SetNeighbour (.Value (Utilities|Map|Find (Variables|Default|GetNeighbours) _array_element)) (Variables|/Game/Game/Data/Direction.Direction_C|GetOppositeDirection _array_element) _returnvalue))))
    (Default|ReplaceTile (Variables|Default|GetTileMapRef) _returnvalue)
    (Actor|DestroyActor)
    (Transformation|AttachActorToActor _returnvalue (Variables|Default|GetTileMapRef) "None" "KeepWorld" "KeepWorld" "KeepWorld" true)))

(fn SetNeighbour
  (params (Direction :type Direction%20Object%20Reference) (NewNeighbour :type Tile%20Object%20Reference))
  (Utilities|Map|Add (Variables|Default|GetNeighbours) Direction NewNeighbour))

(fn CanPlayerEnter
  (params (Player :type Player%20Pawn%20Object%20Reference) (From :type Tile%20Object%20Reference))
  (return false))

(fn GetNextTile
  (params (Player :type Player%20Pawn%20Object%20Reference) (From :type Tile%20Object%20Reference))
  (return 0))