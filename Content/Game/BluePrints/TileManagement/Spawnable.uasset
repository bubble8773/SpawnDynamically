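; Spawnable is a tile actor that marks whether a building can occupy it and spawns that building.
; On BeginPlay it gives its plane a dynamic material, tinted green when CanSpawnBuilding is true and red otherwise.
; A green tile also spawns the Building class at its own transform.
; CanPlayerEnter admits players only when CanSpawnBuilding is false, so building tiles block entry.
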(event EventBeginPlay
  (bind _plane (Variables|Default|GetPlane))
  (|CallParentFunction)
  (bind _returnvalue (Rendering|Material|CreateDynamicMaterialInstance _plane 0 "/Game/Game/Mat/SpawnableMat.SpawnableMat" "None" :!class /Script/Engine.PrimitiveComponent))
  (Rendering|Material|SetMaterial _plane 0 _returnvalue)
  (if (Variables|Default|GetcanSpawnBuilding)
    (Rendering|Material|SetVectorParameterValue _returnvalue "Base Color" "(R=0.065100,G=0.947917,B=0.024910,A=1.000000)" :!class /Script/Engine.MaterialInstanceDynamic)
    (Game|SpawnActorfromClass "/Game/Game/BluePrints/Building.Building_C" (Transformation|GetActorTransform) "Undefined" 0 0)
    (else
      (Rendering|Material|SetVectorParameterValue _returnvalue "Base Color" "(R=0.744792,G=0.000000,B=0.000000,A=1.000000)" :!class /Script/Engine.MaterialInstanceDynamic))))

(event Collision|EventActorBeginOverlap
  (params (OtherActor :type Actor%20Object%20Reference))
  (|CallParentFunction OtherActor) ; This node is disabled and will not be called.\nDrag off pins to build functionality.
)

(event EventTick
  (params (DeltaSeconds :type Float%20%28single-precision%29))
  (|CallParentFunction DeltaSeconds) ; This node is disabled and will not be called.\nDrag off pins to build functionality.
)

(fn ConstructionScript
  (|CallParentFunction))

(fn CanPlayerEnter
  (params (Player :type Player%20Pawn%20Object%20Reference) (From :type Tile%20Object%20Reference))
  (return (not (Variables|Default|GetcanSpawnBuilding))))