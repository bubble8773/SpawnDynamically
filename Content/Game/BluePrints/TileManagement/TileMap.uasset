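; TileMap is an actor that owns the game's tile grid as a flat, row-major array with coordinate lookup, bounds checks and tile replacement.
; ResetMap rebuilds the grid with border and fill tile types, attaching each tile and linking neighbours once all exist.
; Grid Y maps to world X.
; On BeginPlay it switches the view to CameraActor and places the PlayerPawn on its spawn tile and direction.
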(event EventBeginPlay
  (bind _returnvalue (Game|Player|GetPlayerPawn 0))
  (Game|Player|SetViewTargetwithBlend (Game|GetPlayerController 0) (Variables|Default|GetCameraActor) 0.0 "VTBlend_Linear" 0.0 false)
  (Transformation|SetActorLocation _returnvalue (Transformation|GetActorLocation (Variables|Default|GetPlayerSpawnTile)) false false)
  (Transformation|SetActorRotation _returnvalue (Variables|/Game/Game/Data/Direction.Direction_C|GetRotation (Variables|Default|GetPlayerSpawnDirection)) true)
  (bind _asplayer_pawn (Utilities|Casting|CastToPlayerPawn _returnvalue))
  (Variables|/Game/Game/BluePrints/PlayerPawn.PlayerPawn_C|SetCurrentTile _asplayer_pawn (Variables|Default|GetPlayerSpawnTile))
  (Variables|/Game/Game/BluePrints/PlayerPawn.PlayerPawn_C|SetCurrentDirection _asplayer_pawn (Variables|Default|GetPlayerSpawnDirection)))

(event Collision|EventActorBeginOverlap
  (params (OtherActor :type Actor%20Object%20Reference)))

(event EventTick
  (params (DeltaSeconds :type Float%20%28single-precision%29)))

(fn ConstructionScript)

(fn CoordtoIndex
  (params (Coord :type Coord%20Structure))
  (return (+ (.x Coord) (* (.y Coord) (Variables|Default|GetWidth)))))

(fn IndextoCoord
  (params (Index :type Integer))
  (bind _width (Variables|Default|GetWidth))
  (return (Utilities|Struct|MakeCoord (Math|Integer|%(Integer) Index _width) (/ Index _width))))

(fn ResetMap
  (bind _tilesize (Variables|Default|GetTileSize))
  (for _array_element (Variables|Default|GetTile)
    (Utilities|IsValid _array_element
      (:Is%20Valid
        (Actor|DestroyActor _array_element))))
  (Utilities|Array|Clear (Variables|Default|GetTile))
  (for _index (range 0 (- (Variables|Default|GetHeight) 1))
    (for _index_2 (range 0 (- (Variables|Default|GetWidth) 1))
      (bind _returnvalue (Game|SpawnActorfromClass (select (CallFunction|IsonBorder (Utilities|Struct|MakeCoord _index_2 _index)) (Variables|Default|GetBorderTileType) (Variables|Default|GetFillTileType)) (Math|Transform|MakeTransform (Math|Vector|MakeVector (* _index _tilesize) (* _index_2 _tilesize) 0.0) "0, 0, 0" "1,1,1") "Undefined" 0 (select (CallFunction|IsonBorder (Utilities|Struct|MakeCoord _index_2 _index)) (Variables|Default|GetBorderTileType) (Variables|Default|GetFillTileType)) (Utilities|Struct|MakeCoord _index_2 _index) 0 self 0))
      (Utilities|Array|Add (Variables|Default|GetTile) _returnvalue)
      (Transformation|AttachActorToActor _returnvalue self "None" "KeepWorld" "KeepWorld" "KeepWorld" true)))
  (for _array_element_2 (Variables|Default|GetTile)
    (Default|FindNeighbours _array_element_2)))

(fn IsonBorder
  (params (Coord :type Coord%20Structure))
  (return (Math|Boolean|ORBoolean (== (.x Coord) 0) (== (.x Coord) (- (Variables|Default|GetWidth) 1)) (== (.y Coord) 0) (== (.y Coord) (- (Variables|Default|GetHeight) 1)))))

(fn IsCoordinRange
  (params (Coord :type Coord%20Structure))
  (return (not (Math|Boolean|ORBoolean (< (.x Coord) 0) (>= (.x Coord) (Variables|Default|GetWidth)) (< (.y Coord) 0) (>= (.y Coord) (Variables|Default|GetHeight))))))

(fn GetTileatCoord
  (params (Coord :type Coord%20Structure))
  (return (Utilities|Array|Get(acopy) (Variables|Default|GetTile) (CallFunction|CoordtoIndex Coord))))

(fn ReplaceTile
  (params (NewTile :type Tile%20Object%20Reference))
  (Utilities|Array|SetArrayElem (Variables|Default|GetTile) (CallFunction|CoordtoIndex (Variables|/Game/Game/BluePrints/TileManagement/Tile.Tile_C|GetCoord NewTile)) NewTile))